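; Player Blueprint for a dog-care game, handling mouse look and the commands the player gives to the dog.
; BeginPlay caches the dog, ball and fade sequence, and an Interact cursor trace shows or hides the HUD UI depending on a dog hit.
; Command events drive Dog_BP reactions with sounds or a walk fade.
; Play throws any held ball by impulse until ReceiveBall restores it, and bites splash the screen red.
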(event `self.ReceiveBeginPlay`
  ;[1 1 1] Temp Show Mouse
  (set `PlayerController.bShowMouseCursor` true (`GameplayStatics.GetPlayerController` 0))
  (bind _outactors (`GameplayStatics.GetAllActorsOfClass` "/Game/DogAssets/Dog_BP.Dog_BP_C"))
  (set `self.Dog BP` (`|GetArrayItem` _outactors))
  (bind _returnvalue (`GameplayStatics.GetActorOfClass` "/Game/Player/Ball_BP.Ball_BP_C"))
  (set `self.Ball BP` _returnvalue)
  (bind (_outactor _returnvalue_2) (`LevelSequencePlayer.CreateLevelSequencePlayer` "/Game/FadeInOut.FadeInOut"))
  (set `self.FadeInOut` _returnvalue_2))

(event `Throw Ball`
  ;[1 1 1] Play With Dog
  (`/Engine/EditorBlueprintResources/StandardMacros.IsValid` (`self.Ball BP`)
    (:`Is Valid`
      (`self.K2_SetActorLocation` (`self.Ball BP`) (`SceneComponent.K2_GetComponentLocation` (`self.Ball Position`)) false false)
      (`PrimitiveComponent.AddImpulse` (`/Game/Player/Ball_BP.Sphere` (`self.Ball BP`)) (* (`KismetMathLibrary.GetForwardVector` (`self.GetControlRotation`)) 500.0) "None" false)
      (set `self.Ball BP` null)
      (set `/Game/DogAssets/Dog_BP.Has Ball Been Thrown` true (`self.Dog BP`)))))

(event `InputAxis|LookUp`
  (params (AxisValue :type "Float (single-precision)"))
  ;[1 1 1] TODO - Add Android support - Look Around
  (`self.AddControllerPitchInput` AxisValue))

(event `InputAxis|LookRight`
  (params (AxisValue :type "Float (single-precision)"))
  ;[1 1 1] TODO - Add Android support - Look Around
  (`self.AddControllerYawInput` AxisValue))

(event `Receive Ball`
  (params (`Ball From Dog` :type "/Game/Player/Ball_BP Object Reference"))
  ;[1 1 1] Play With Dog
  (set `self.Ball BP` `Ball From Dog`))

(event `InputAction|Interact`
  (params (Key :type "Key Structure"))
  (bind _returnvalue (`PlayerController.GetHUD` (`GameplayStatics.GetPlayerController` 0)))
  ;[1 1 1] Line Trace for Dog
  (:`Pressed`
    (cast `/Game/DogAssets/Dog_BP` (`.HitActor` (`GameplayStatics.BreakHitResult` (`PlayerController.GetHitResultUnderCursorByChannel` (`GameplayStatics.GetPlayerController` 0) "TraceTypeQuery1" true)))
      (:`then`
        (bind _asplayer_hud (cast `/Game/Player/Player_HUD` _returnvalue))
        (`/Game/Player/Player_HUD.Show UI` _asplayer_hud))
      (:`CastFailed`
        (bind _asplayer_hud_2 (cast `/Game/Player/Player_HUD` _returnvalue))
        (`/Game/Player/Player_HUD.Hide UI` _asplayer_hud_2)))))

(event `Get Bitten`
  ;[1 1 1] Get Bitten
  (bind _asplayer_controller_bp (cast `/Game/Player/PlayerController_BP` (`GameplayStatics.GetPlayerController` 0)))
  (`/Game/Player/PlayerController_BP.Splash Red Screen` _asplayer_controller_bp))

(event `Hit Dog`
  ;[1 1 1] Hit Dog
  (`/Game/DogAssets/Dog_BP.Get Hit` (`self.Dog BP`))
  (`/Game/DogAssets/Dog_BP.Learn To Be Clean` (`self.Dog BP`)))

(event `Scold Dog`
  ;[1 1 1] Scold Dog
  (`GameplayStatics.PlaySound2D` "/Game/DogAssets/Sounds/No_Cue.No_Cue" 1.0 1.0 0.0 null null)
  (`KismetSystemLibrary.Delay` 0.4)
  (`/Game/DogAssets/Dog_BP.React To Scold` (`self.Dog BP`)))

(event `Pat Dog`
  ;[1 1 1] Pat Dog
  (`/Game/DogAssets/Dog_BP.Receive Pat` (`self.Dog BP`)))

(event `Walk Dog`
  ;[1 1 1] Walk Dog
  (`/Game/DogAssets/Dog_BP.Check Player's Action` (`self.Dog BP`) "NewEnumerator3")
  (`/Game/DogAssets/Dog_BP.Go For a Walk` (`self.Dog BP`))
  (`MovieSceneSequencePlayer.Play` (`self.FadeInOut`)))

(event `Whistle`
  ;[1 1 1] Whistle
  (`GameplayStatics.PlaySoundAtLocation` "/Game/DogAssets/Sounds/Whistle_Cue.Whistle_Cue" (0.0 0.0 0.0) (struct) 1.0 1.0 0.0 null null null)
  (`/Game/DogAssets/Dog_BP.React To Whistle` (`self.Dog BP`)))

(event `Feed`
  ;[1 1 1] Feed
  (`/Game/DogAssets/Dog_BP.Check Player's Action` (`self.Dog BP`) "NewEnumerator0")
  (`/Game/DogAssets/Dog_BP.Eat` (`self.Dog BP`)))

(event `Play With Dog`
  ;[1 1 1] Play WIth Dog
  (`/Game/DogAssets/Dog_BP.Check Player's Action` (`self.Dog BP`) "NewEnumerator1")
  (if (`KismetSystemLibrary.IsValid` (`self.Ball BP`))
    (`self.Throw Ball`)
    (`KismetSystemLibrary.Delay` 0.5)
    (`/Game/DogAssets/Dog_BP.React To Ball` (`self.Dog BP`))
    (else
      (`/Game/DogAssets/Dog_BP.React To Ball` (`self.Dog BP`)))))

(fn `UserConstructionScript`)