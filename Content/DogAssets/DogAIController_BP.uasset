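; AI controller for the dog pawn that drives it with the dog behaviour tree.
; On BeginPlay it runs the tree and caches the controlled pawn as Dog_BP.
; A SetIsPottyTrained event writes the potty-trained flag to the blackboard, along with the dog's player reference as the Player Character key.
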(event `Set IsPottyTrained`
  (params (IsPottyTrained :type Boolean))
  (`BlackboardComponent.SetValueAsBool` (`AIBlueprintHelperLibrary.GetBlackboard` null) "IsPottyTrained" IsPottyTrained)
  (`BlackboardComponent.SetValueAsObject` (`AIBlueprintHelperLibrary.GetBlackboard` null) "Player Character" (`/Game/DogAssets/Dog_BP.Player BP` (`self.Dog BP`))))

(event `self.ReceiveBeginPlay`
  (`self.RunBehaviorTree` self "/Game/DogAssets/AILogic/DogBehaviourTree.DogBehaviourTree")
  (bind _asdog_bp (cast `/Game/DogAssets/Dog_BP` (`self.K2_GetPawn`)))
  (set `self.Dog BP` _asdog_bp))

(fn `UserConstructionScript`)