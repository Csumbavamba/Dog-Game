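; Pitbull dog character that acts on random needs and reacts to the player's whistles, pats, scolds, hits and thrown balls.
; A Tick-driven delay picks HighestNeed from a shrinking list, replacing disconnected need-decay logic; excessive hits override it.
; Events drive montages and AI moves to player, ball, bowl or door, with several finishing by choosing another need.
; Scolding uses the briefly locked last behaviour to set potty training on the AI controller.
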(event `self.ReceiveBeginPlay`
  (`|ExecutionSequence`
    (:`then_0`
      ;[1 1 1] Setup Need Requirements
      (set `self.Times Hit` 0)
      (set `self.Feed Level` (`self.Max Feed Level`))
      (set `self.Excitement Level` (`self.Max Excitement Level`))
      (`self.Set Speed` (`self.WalkingSpeed`))
      (bind _output_get (set `self.BehaviourTime` 20.0))
      (bind _output_get_2 (set `self.MaxPoopLevel` (- _output_get 5.0)))
      (set `self.PoopLevel` _output_get_2))
    (:`then_1`
      ;[1 1 1] Setup Dog
      (bind _returnvalue (`GameplayStatics.GetActorOfClass` "/Game/Player/Player_BP.Player_BP_C"))
      (set `self.Player BP` _returnvalue)
      (bind _aspitbull_abp (cast `/Game/DogAssets/Pitbull_ABP` (`SkeletalMeshComponent.GetAnimInstance` (`self.Mesh`))))
      (set `self.Anim Instance` _aspitbull_abp)
      (bind _returnvalue_2 (`GameplayStatics.GetActorOfClass` "/Game/Player/Ball_BP.Ball_BP_C"))
      (set `self.Ball BP` _returnvalue_2)
      (bind _returnvalue_3 (`GameplayStatics.GetActorOfClass` "/Game/DogAssets/ObjectsForDog/Door_BP.Door_BP_C"))
      (set `self.Door BP` _returnvalue_3)
      (bind _returnvalue_4 (`GameplayStatics.GetActorOfClass` "/Game/DogAssets/ObjectsForDog/TestBowl_BP.TestBowl_BP_C"))
      (set `self.Bowl BP` _returnvalue_4)
      (bind _asdog_aicontroller_bp (cast `/Game/DogAssets/DogAIController_BP` (`AIBlueprintHelperLibrary.GetAIController` self)))
      (set `self.AI Controller BP` _asdog_aicontroller_bp))
    (:`then_2`
      ;[1 1 1] Add Potential Needs
      (`self.Choose New Behaviour`))))

(event `self.ReceiveTick`
  (params (DeltaSeconds :type "Float (single-precision)"))
  ;[1 1 1] Tick - Chosing Random Behaviours every 20 seconds
  (if (> (`self.Times Hit`) (`self.MaxAcceptedHits`))
    (set `self.Highest Need` "NewEnumerator5")
    (elif (`|EnumInequality` (`self.Highest Need`) "NewEnumerator3")
      (`KismetSystemLibrary.Delay` (`self.BehaviourTime`))
      (if (!= (`KismetArrayLibrary.Array_Length` (`self.Potential Needs`)) 0)
        (`self.Choose New Behaviour`)
        (else
          (`KismetSystemLibrary.PrintString` "TODO Add End Screen")))
      (else
        (set `self.PoopLevel` (- (`self.PoopLevel`) (`GameplayStatics.GetWorldDeltaSeconds`)))))))

(event `Choose New Behaviour`
  (bind _returnvalue (`KismetMathLibrary.RandomInteger` (- (`KismetArrayLibrary.Array_Length` (`self.Potential Needs`)) 1)))
  ;[1 1 1] Choose New Behaviour
  (set `self.Highest Need` (`|GetArrayItem` (`self.Potential Needs`) _returnvalue))
  (bind _output_get (set `self.BehaviourToRemove` _returnvalue))
  (`KismetArrayLibrary.Array_Remove` (`self.Potential Needs`) _output_get)
  (`KismetSystemLibrary.PrintString` (`KismetStringLibrary.Conv_IntToString` (`KismetArrayLibrary.Array_Length` (`self.Potential Needs`)))))

(event `React To Scold`
  ;[1 1 1] Receive Scold
  (`self.PlayAnimMontage` "/Game/DogAssets/Animations/PitbullSad_Anim_Montage.PitbullSad_Anim_Montage")
  (`self.Get Scolded`))

(event `React To Whistle`
  ;[1 1 1] React To Whistle
  (if (and (`self.CanMove`) (`|EnumEquality` (`self.Highest Need`) "NewEnumerator4"))
    (`|AIMoveTo` self (0.0 0.0 0.0) (`self.Player BP`) 75.0)))

(event `Receive Pat`
  ;[1 1 1] Receive Pat
  (set `self.HasBeenPatted` true)
  (`self.PlayAnimMontage` "/Game/DogAssets/Animations/PitbullHappy_Anim_Montage.PitbullHappy_Anim_Montage"))

(event `Get Hit`
  ;[1 1 1] Get Hit
  (`GameplayStatics.PlaySound2D` "/Game/DogAssets/Sounds/Slap_Cue.Slap_Cue" 1.0 1.0 0.0 null null)
  (if (`|EnumInequality` (`self.Highest Need`) "NewEnumerator5")
    (`self.PlayAnimMontage` (select `int` (`KismetMathLibrary.RandomInteger` 2) :`0` "/Game/DogAssets/Animations/PitbullAggressiveBeingHit1_Anim_Montage.PitbullAggressiveBeingHit1_Anim_Montage" :`1` "/Game/DogAssets/Animations/PitbullAggressiveBeingHit2_Anim_Montage.PitbullAggressiveBeingHit2_Anim_Montage" :`2` "/Game/DogAssets/Animations/PitbullAggressiveBeingHit3_Anim_Montage.PitbullAggressiveBeingHit3_Anim_Montage" :!type "AnimMontage Object Reference"))
    (`/Engine/EditorBlueprintResources/StandardMacros.IncrementInt` (`self.Times Hit`)
      (:`  `
        (`|ExecutionSequence`
          (:`then_0`
            (`self.Become Pissed`))
          (:`then_1`
            (if (or (>= (`self.Times Hit`) 3) (<= (`self.MaxAcceptedHits`) 3))
              (`KismetSystemLibrary.Delay` 0.5)
              (if (`|EnumInequality` (`self.Highest Need`) "NewEnumerator5")
                (`self.PlayAnimMontage` "/Game/DogAssets/Animations/PitbullAggressiveBarking_Anim_Montage.PitbullAggressiveBarking_Anim_Montage")))))))))

(event `Become Pissed`
  ;[1 1 1] Become Pissed
  (if (`self.IsPissed`)
    (set `self.PissedTime` (+ (`self.PissedTime`) 15.0))
    (else
      (set `self.IsPissed` true)
      (set `self.PissedTime` 15.0))))

(event `Eat`
  ;[1 1 1] Eat
  (bind _returnvalue (`GameplayStatics.SpawnSound2D` "/Game/DogAssets/Sounds/Eating_Cue.Eating_Cue" 1.0 1.0 0.0 null))
  (set `self.Eating Sound` _returnvalue)
  (`self.PlayAnimMontage` "/Game/DogAssets/Animations/PitbullEat_Anim_Montage.PitbullEat_Anim_Montage"))

(event `Go For a Walk`
  ;[1 1 1] Go For A Walk
  (set `self.PoopLevel` (`self.MaxPoopLevel`))
  (`self.Choose New Behaviour`))

(event `Finish Eating`
  ;[1 1 1] Finish Eating
  (set `self.Feed Level` (`self.Max Feed Level`))
  (set `self.PoopLevel` (- (`self.PoopLevel`) (/ (`self.MaxPoopLevel`) 5.0)))
  (`/Engine/EditorBlueprintResources/StandardMacros.IsValid` (`self.Eating Sound`)
    (:`Is Valid`
      (`AudioComponent.Stop` (`self.Eating Sound`))
      (`self.Choose New Behaviour`))))

(event `React To Ball`
  ;[1 1 1] Playing with the Ball
  ;;[0.05127 0 0.4072] React To Thrown Ball
  (if (`self.IsPissed`)
    (`self.PlayAnimMontage` "/Game/DogAssets/Animations/PitbullAggressiveBarking_Anim_Montage.PitbullAggressiveBarking_Anim_Montage")
    (elif (`|EnumEquality` (`self.Highest Need`) "NewEnumerator4")
      (`self.Run After Ball`))))

(event `Bring Ball Back`
  ;[1 1 1] Playing with the Ball
  ;;[0.1243 0 1] Bring Ball Back
  (`|AIMoveTo` self (0.0 0.0 0.0) (`self.Player BP`) 75.0
    (:`OnSuccess`
      (`self.HandOverBall`))))

(event `Run After Ball`
  ;[1 1 1] Playing with the Ball
  ;;[0.05127 0 0.4072] Run After Ball
  (`self.Set Speed` (`self.RunningSpeed`))
  (`/Engine/EditorBlueprintResources/StandardMacros.IsValid` (`self.Ball BP`)
    (:`Is Valid`
      (`|AIMoveTo` self (0.0 0.0 0.0) (`self.Ball BP`) 75.0
        (:`OnSuccess`
          _)
        (:`OnFail`
          _))
      (if (`self.Has Ball Been Thrown`)
        (`self.K2_DestroyActor` (`self.Ball BP`))
        (set `self.Has Ball Been Thrown` false)
        (`self.Bring Ball Back`)
        (else
          (`self.Bring Ball Back`))))
    (:`Is Not Valid`
      (`self.Bring Ball Back`))))

(event `Focus Player`
  (bind (_returnvalue_roll _returnvalue_pitch _returnvalue_yaw) (`KismetMathLibrary.BreakRotator` (`KismetMathLibrary.FindLookAtRotation` (`self.K2_GetActorLocation`) (`self.K2_GetActorLocation` (`self.Player BP`)))))
  ;[1 1 1] Focus Player
  (`SceneComponent.K2_SetWorldRotation` (`self.CapsuleComponent`) (`KismetMathLibrary.MakeRotator` 0.0 0.0 _returnvalue_yaw) false false))

(event `Bark`
  ;[1 1 1] Bark
  (`self.PlayAnimMontage` "/Game/DogAssets/Animations/PitbullIdleBarking_Anim_Montage.PitbullIdleBarking_Anim_Montage"))

(event `Learn To Be Clean`
  ;[1 1 1] Learn To Stay Clean
)

(event `Ask For Food`
  ;[1 1 1] Go To Food Bowl
  (if (`self.CanMove`)
    (`|AIMoveTo` self (0.0 0.0 0.0) (`self.Bowl BP`) 75.0)))

(event `Set Movement Enabled`
  (params (CanMove :type Boolean))
  ;[1 1 1] Stop Movement
  (bind _output_get (set `self.CanMove` CanMove))
  (if (not _output_get)
    (`MovementComponent.StopMovementImmediately` (`self.CharacterMovement`))
    (`self.Set Speed` (`self.WalkingSpeed`))))

(event `Request Walking`
  ;[1 1 1] Ask For Walking
  (if (`self.CanMove`)
    (`|AIMoveTo` self (0.0 0.0 0.0) (`self.Door BP`) 75.0)))

(event `Take a Poop`
  ;[1 1 1] Take a Poop
  (`self.PlayAnimMontage` "/Game/DogAssets/Animations/PitbullPoop_Anim_Montage.PitbullPoop_Anim_Montage")
  (set `self.PoopLevel` (`self.MaxPoopLevel`))
  (`KismetSystemLibrary.Delay` 1.0)
  (`self.Choose New Behaviour`))

(event `Growl`
  ;[1 1 1] Growl
  (`self.PlayAnimMontage` "/Game/DogAssets/Animations/PitbullAggressiveIdle_Anim_Montage.PitbullAggressiveIdle_Anim_Montage" 0.4))

(event `Jump Around`
  ;[1 1 1] Jump Until Patted
  (if (`self.HasBeenPatted`)
    (set `self.HasBeenPatted` false)
    (else
      (`|PlayMontage` (`self.Mesh`) "/Game/DogAssets/Animations/PitbullJump_Anim_Montage.PitbullJump_Anim_Montage"
        (:`OnBlendOut`
          (`self.Jump Around`))))))

(event `Attack Player`
  ;[1 1 1] Get Bitten
  (`self.PlayAnimMontage` "/Game/DogAssets/Animations/PitbullAggressiveAttack2_Anim_Montage.PitbullAggressiveAttack2_Anim_Montage")
  (`KismetSystemLibrary.Delay` 1.0)
  (`/Game/Player/Player_BP.Get Bitten` (`self.Player BP`))
  (set `self.MaxAcceptedHits` 3)
  (set `self.Times Hit` 0)
  (`self.Choose New Behaviour`))

(event `Get Scolded`
  (switch `/Game/DogAssets/EDogBehaviour` (`self.Last Behaviour`)
    (:`NewEnumerator0`
      ;[1 1 1] If He Shit himself - Prefer Walk
      (`/Game/DogAssets/DogAIController_BP.Set IsPottyTrained` (`self.AI Controller BP`) true))
    (:`NewEnumerator1`
      ;[1 1 1] If he went for a walk - Prefer Shit
      (`/Game/DogAssets/DogAIController_BP.Set IsPottyTrained` (`self.AI Controller BP`) false))))

(event `Save Behaviour For 5 Seconds`
  (params (`Dog Behaviour` :type "/Game/DogAssets/EDogBehaviour Enum" :default "NewEnumerator0"))
  ;[1 1 1] Save Behaviour For 5 seconds
  (if (`self.Need Saved`)
    (set `self.Temporary Saved Behaviour` `Dog Behaviour`)
    (`KismetSystemLibrary.Delay` 5.0)
    (set `self.Need Saved` false)
    (`self.Save Behaviour For 5 Seconds` (`self.Temporary Saved Behaviour`))
    (else
      (bind _output_get (set `self.Last Behaviour` `Dog Behaviour`))
      (set `self.Need Saved` true)
      (`KismetSystemLibrary.PrintString` (`|GetEnumeratorNameAsString` _output_get))
      (`KismetSystemLibrary.Delay` 5.0)
      (set `self.Need Saved` false))))

(fn `Check If Still Bored`
  (if (<= (`self.TimesPlayed`) 4)
    (`/Engine/EditorBlueprintResources/StandardMacros.IncrementInt` (`self.TimesPlayed`))
    (else
      (set `self.TimesPlayed` 0)
      (set `self.Excitement Level` (`self.Max Excitement Level`)))))

(fn `HandOverBall`
  (`/Engine/EditorBlueprintResources/StandardMacros.IsValid` (`self.Ball BP`)
    (:`Is Not Valid`
      (bind _returnvalue (`|SpawnActorFromClass` "/Game/Player/Ball_BP.Ball_BP_C" (`KismetMathLibrary.MakeTransform` (+ (`self.K2_GetActorLocation`) (* (`KismetMathLibrary.GetForwardVector` (`self.GetControlRotation`)) 50.0)) (struct) (0.1 0.1 0.1)) "Undefined" "OverrideRootScale" null null))
      (bind _output_get (set `self.Ball BP` _returnvalue))
      (`/Game/Player/Player_BP.Receive Ball` (`self.Player BP`) _output_get)
      (`self.Check If Still Bored`)
      (`self.Set Speed` (`self.WalkingSpeed`)))))

(fn `Set Speed`
  (params (MaxWalkSpeed :type "Float (double-precision)"))
  (set `CharacterMovementComponent.MaxWalkSpeed` MaxWalkSpeed (`self.CharacterMovement`)))

(fn `UserConstructionScript`)