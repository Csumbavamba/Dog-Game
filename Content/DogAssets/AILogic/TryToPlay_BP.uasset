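; Behavior tree task that has the dog fetch a ball and bring it to the player.
; It sets the dog to running speed and moves it to the ball, destroying the ball if flagged as thrown, then returns to the player to hand it over and finish successfully.
; Without a valid ball it heads straight to the player, and failed moves continue exactly like successful ones.
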(event `self.ReceiveExecuteAI`
  (params (OwnerController :type "AIController Object Reference") (ControlledPawn :type "Pawn Object Reference"))
  (bind _asdog_bp (cast `/Game/DogAssets/Dog_BP` ControlledPawn))
  (bind _output_get (set `self.Dog BP` _asdog_bp))
  (set `self.Ball BP` (`/Game/DogAssets/Dog_BP.Ball BP` _output_get))
  (`/Game/DogAssets/Dog_BP.Set Speed` (`self.Dog BP`) (`/Game/DogAssets/Dog_BP.RunningSpeed` _output_get))
  (`/Engine/EditorBlueprintResources/StandardMacros.IsValid` (`self.Ball BP`)
    (:`Is Valid`
      (`|AIMoveTo` (`self.Dog BP`) (0.0 0.0 0.0) (`self.Ball BP`) 75.0
        (:`OnSuccess`
          _)
        (:`OnFail`
          _))
      (if (`/Game/DogAssets/Dog_BP.Has Ball Been Thrown` (`self.Dog BP`))
        (`Actor.K2_DestroyActor` (`self.Ball BP`))
        (set `/Game/DogAssets/Dog_BP.Has Ball Been Thrown` false (`self.Dog BP`))
        (`self.Bring Ball Back`)
        (else
          (`self.Bring Ball Back`))))
    (:`Is Not Valid`
      (`self.Bring Ball Back`))))

(event `Bring Ball Back`
  ;[1 1 1] Bring Ball Back
  (`|AIMoveTo` (`self.Dog BP`) (0.0 0.0 0.0) (`/Game/DogAssets/Dog_BP.Player BP` (`self.Dog BP`)) 75.0
    (:`OnSuccess`
      _)
    (:`OnFail`
      _))
  (`/Game/DogAssets/Dog_BP.HandOverBall` (`self.Dog BP`))
  (`self.FinishExecute` true))