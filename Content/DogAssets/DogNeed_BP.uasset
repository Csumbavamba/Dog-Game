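; Dog need Blueprint that chooses which sub-behaviour the dog does for this need, learning preferences from feedback.
; GetFeedback writes the received feedback to the latest behaviour's IsPreferred flag.
; GetBehaviourToDo appends flagged sub-behaviours to PreferredBehaviours, never clearing it here, then picks randomly from that list, or from all sub-behaviours if empty.
; GetRandomBehaviour passes length minus one to RandomInteger, whose maximum is exclusive, so the last element is skipped in multi-item lists.
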(event `Get Feedback`
  (params (Feedback :type Boolean))
  ;[1 1 1] Receive Feedback
  (set `/Game/DogAssets/Behaviour_BP.IsPreferred` Feedback (`self.Latest Behaviour`)))

(event `Get Behaviour To Do`
  ;[1 1 1] Find Behaviour To Do
  (for _array_element (`self.SubBehaviours`)
    (if (`/Game/DogAssets/Behaviour_BP.IsPreferred` _array_element)
      (`KismetArrayLibrary.Array_Add` (`self.Preferred Behaviours`) _array_element)))
  (if (== (`KismetArrayLibrary.Array_Length` (`self.Preferred Behaviours`)) 0)
    (bind _behaviour (`self.GetRandomBehaviour` (`self.SubBehaviours`)))
    (set `self.Preferred Behaviour` _behaviour)
    (else
      (bind _behaviour_2 (`self.GetRandomBehaviour` (`self.Preferred Behaviours`)))
      (set `self.Preferred Behaviour` _behaviour_2))))

(fn `GetRandomBehaviour`
  (params (Behaviours :type "Array of /Game/DogAssets/Behaviour_BP Object Reference"))
  (returns (Behaviour :type "/Game/DogAssets/Behaviour_BP Object Reference"))
  (return (`|GetArrayItem` Behaviours (`KismetMathLibrary.RandomInteger` (- (`KismetArrayLibrary.Array_Length` Behaviours) 1)))))